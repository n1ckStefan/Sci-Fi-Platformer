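; BP_Collectable is a pickup that adds score to BP_ThirdPersonCharacter when it overlaps the sphere, then destroys itself.
; CollectableIndex selects the score value, plus the colour and scale the construction script applies to both Niagara effects.
; The first overlap updates the count, shows a pop-up and swaps the idle effect for a burst.
; A timeline keeps feeding the player's position into the burst for an absorb effect until the actor is destroyed.
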(event OnComponentBeginOverlap(Sphere)
  (params (OverlappedComponent :type Primitive%20Component%20Object%20Reference) (OtherActor :type Actor%20Object%20Reference) (OtherComp :type Primitive%20Component%20Object%20Reference) (OtherBodyIndex :type Integer) (bFromSweep :type Boolean) (SweepResult :type Hit%20Result%20Structure%20%28by%20ref%29))
  (Utilities|FlowControl|DoOnce false
    (:Completed
      (bind _asbp_third_person_character (Utilities|Casting|CastToBP_ThirdPersonCharacter OtherActor))
      (CallFunction|AddCollectableScore)
      (Components|DestroyComponent (Variables|Default|GetCollectable))
      (Components|Activation|Activate (Variables|Default|GetCollectableBurst) false)
      (Class|NiagaraComponent|SetVariablePosition (Variables|Default|GetCollectableBurst) "PlayerPos" (Transformation|GetWorldLocation (Variables|/Script/Engine.Character|GetMesh _asbp_third_person_character)))
      ;[0.03577 0.05482 0.15 0.5] Pass player position into niagara to create the absorb effect
      (Timeline|Timeline Play
        (:Update
          (bind _returnvalue (Actor|GetActorOfClass "/Game/ThirdPerson/Blueprints/BP_ThirdPersonCharacter.BP_ThirdPersonCharacter_C"))
          (Class|NiagaraComponent|SetVariablePosition (Variables|Default|GetCollectableBurst) "PlayerPos" (Transformation|GetWorldLocation (Variables|/Script/Engine.Character|GetMesh _returnvalue))))
        (:Finished
          (Actor|DestroyActor))))))

(event Custom|Add%20Collectable%20Score
  (bind _output_get (Variables|/Game/ThirdPerson/Blueprints/BP_ThirdPersonCharacter.BP_ThirdPersonCharacter_C|SetCollectableCount (stale OnComponentBeginOverlap(Sphere) _asbp_third_person_character) (+ (Utilities|Array|Get(acopy) (Variables|Default|GetCollectableValue) (Variables|Default|GetCollectableIndex)) (Variables|/Game/ThirdPerson/Blueprints/BP_ThirdPersonCharacter.BP_ThirdPersonCharacter_C|GetCollectableCount (stale OnComponentBeginOverlap(Sphere) _asbp_third_person_character)))))
  (Development|PrintString (Utilities|String|ToString(Integer) _output_get))
  (Default|ShowCollectablePopUp (stale OnComponentBeginOverlap(Sphere) _asbp_third_person_character)))

(fn ConstructionScript
  (bind _colour (Variables|Default|GetColour))
  (bind _collectableindex (Variables|Default|GetCollectableIndex))
  (bind _output (Utilities|Array|Get(acopy) _colour _collectableindex))
  (Niagara|SetNiagaraVariable(LinearColor) (Variables|Default|GetCollectableBurst) "Colour" _output)
  (Niagara|SetNiagaraVariable(LinearColor) (Variables|Default|GetCollectable) "Linear Color" _output)
  (Niagara|SetNiagaraVariable(Float) (Variables|Default|GetCollectableBurst) "Scale" (Utilities|Array|Get(acopy) (Variables|Default|GetCollectableScale) (Variables|Default|GetCollectableIndex))))