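; Patrolling slime enemy that the player defeats on contact with its trigger capsule, getting bounced upward.
; It loops AIMoveTo between its start position and a fixed offset until hit, then squishes, plays VFX and sound, fades via material Timeline and destroys itself.
; A separate reaction collider triggers a companion AI reaction, re-armed after a delay.
; The construction script picks the slime material by Index and tints both effects with Colour1.
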(event OnComponentBeginOverlap(Capsule)
  (params (OverlappedComponent :type Primitive%20Component%20Object%20Reference) (OtherActor :type Actor%20Object%20Reference) (OtherComp :type Primitive%20Component%20Object%20Reference) (OtherBodyIndex :type Integer) (bFromSweep :type Boolean) (SweepResult :type Hit%20Result%20Structure%20%28by%20ref%29))
  (bind _asbp_third_person_character (Utilities|Casting|CastToBP_ThirdPersonCharacter OtherActor))
  (Utilities|FlowControl|DoOnce false
    (:Completed
      (Components|Animation|PlayAnimation (Variables|Character|GetMesh) "/Game/Art/Characters/Slime/Anims/enemysquish_Montage.enemysquish_Montage" false)
      (Components|Activation|Activate (Variables|Default|GetHitVFX) false)
      (Audio|PlaySound2D "/Game/Sounds/freesound_community-toy-button-105724.freesound_community-toy-button-105724" 1.0 1.0 0.0 0 0)
      (Character|LaunchCharacter _asbp_third_person_character "0.000000,0.000000,700.000000" true true)
      (Collision|SetCollisionEnabled (Variables|Collision|GetCapsuleComponent) "NoCollision")
      (Variables|/Game/ThirdPerson/Blueprints/BP_ThirdPersonCharacter.BP_ThirdPersonCharacter_C|SetJumpCount _asbp_third_person_character 1)
      (Utilities|FlowControl|Delay 0.3)
      (Audio|Components|Audio|Stop (Variables|Character|GetMesh))
      (Components|Activation|Activate (Variables|Default|GetNS_Fade) false)
      (bind _fade (Timeline|Timeline Play)
        (:Update
          (Rendering|Material|SetScalarParameterValueonMaterials (Variables|Character|GetMesh) "Fade" _fade))
        (:Finished
          (Actor|DestroyActor))))))

(event OnComponentBeginOverlap(ReactionCollider)
  (params (OverlappedComponent :type Primitive%20Component%20Object%20Reference) (OtherActor :type Actor%20Object%20Reference) (OtherComp :type Primitive%20Component%20Object%20Reference) (OtherBodyIndex :type Integer) (bFromSweep :type Boolean) (SweepResult :type Hit%20Result%20Structure%20%28by%20ref%29))
  (Utilities|Casting|CastToBP_ThirdPersonCharacter OtherActor)
  (Utilities|FlowControl|DoOnce false
    (:Completed
      (bind _returnvalue (Actor|GetActorOfClass "/Game/NickTech/AI/Companion/AI_CompanionNew.AI_CompanionNew_C"))
      (Default|ChangeReaction _returnvalue 3.0))))

(event OnComponentEndOverlap(ReactionCollider)
  (params (OverlappedComponent :type Primitive%20Component%20Object%20Reference) (OtherActor :type Actor%20Object%20Reference) (OtherComp :type Primitive%20Component%20Object%20Reference) (OtherBodyIndex :type Integer))
  (Utilities|FlowControl|Delay 5.0)
  (Utilities|FlowControl|DoOnce false) ; enters at Reset
)

(event Custom|Patrol
  (AI|AIMoveTo self (+ (Variables|Default|GetStartPosition) "0.000000,-100.000000,0.000000") 0 5.0 false :!label _label
    (:OnSuccess
      _)
    (:OnFail
      _))
  (AI|AIMoveTo self (Variables|Default|GetStartPosition) 0 5.0 false
    (:OnSuccess
      (goto _label))
    (:OnFail
      (goto _label))))

(event EventBeginPlay
  (Variables|Default|SetStartPosition (Transformation|GetActorLocation))
  (CallFunction|Patrol))

(fn ConstructionScript
  (if (== (Variables|Default|GetIndex) 0.0)
    (Rendering|Material|SetMaterial (Variables|Character|GetMesh) 1 "/Game/Art/Characters/Slime/M_Slime.M_Slime")
    (Niagara|SetNiagaraVariable(LinearColor) (Variables|Default|GetHitVFX) "Linear Color" (Variables|Default|GetColour1) :!label _label)
    (Niagara|SetNiagaraVariable(LinearColor) (Variables|Default|GetNS_Fade) "Colour" (Variables|Default|GetColour1))
    (elif (== (Variables|Default|GetIndex) 1.0)
      (Rendering|Material|SetMaterial (Variables|Character|GetMesh) 1 "/Game/Art/Characters/Slime/M_Slime1.M_Slime1")
      (goto _label)
      (elif (== (Variables|Default|GetIndex) 2.0)
        (Rendering|Material|SetMaterial (Variables|Character|GetMesh) 1 "/Game/Art/Characters/Slime/M_Slime2.M_Slime2")
        (goto _label)))))