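; A level exit portal that stays locked until the player has collected enough orbs, then warps them to another level.
; Tick reads the collectable count from BP_Gameinstance, updates a count/needed text, and swaps the cube between locked and hue-shifted open materials.
; Overlapping while unlocked triggers a Niagara fade, sound, input lock and timeline-driven mesh fade.
; It then opens the target level, passing WarpPointTag as a SpawnTag option.
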(event OnComponentBeginOverlap(BoxCollision)
  (params (OverlappedComponent :type Primitive%20Component%20Object%20Reference) (OtherActor :type Actor%20Object%20Reference) (OtherComp :type Primitive%20Component%20Object%20Reference) (OtherBodyIndex :type Integer) (bFromSweep :type Boolean) (SweepResult :type Hit%20Result%20Structure%20%28by%20ref%29))
  (bind _asbp_third_person_character (Utilities|Casting|CastToBP_ThirdPersonCharacter OtherActor))
  (if (not (Variables|Default|GetLocked))
    (Components|Activation|Activate (Variables|/Game/ThirdPerson/Blueprints/BP_ThirdPersonCharacter.BP_ThirdPersonCharacter_C|GetNS_Fade _asbp_third_person_character) false)
    (Utilities|FlowControl|Delay 0.5)
    (Audio|PlaySound2D "/Game/Sounds/freesound_community-magic-smite-6012.freesound_community-magic-smite-6012" 1.0 1.0 0.0 0 0)
    (Input|SetIgnoreMoveInput (Game|GetPlayerController 0) true)
    (bind _newtrack_0 (Timeline|Timeline Play)
      (:Update
        (bind _returnvalue (Actor|GetActorOfClass "/Game/ThirdPerson/Blueprints/BP_ThirdPersonCharacter.BP_ThirdPersonCharacter_C"))
        (Rendering|Material|SetScalarParameterValueonMaterials (Variables|/Script/Engine.Character|GetMesh _returnvalue) "Fade" _newtrack_0))
      (:Finished
        (CallFunction|OpenLevel)))))

(event Custom|Open%20Level
  (Utilities|FlowControl|Delay 0.2)
  (Game|OpenLevel(byObjectReference) (Variables|Default|GetLevel) false (Utilities|String|Append "SpawnTag=" (Variables|Default|GetWarpPointTag))))

(event Custom|ShowText
  (if (> (Variables|Default|GetOrbs%20Needed) 0)
    (bind _count (Default|LoadCollectableCount (.AsBP%20Gameinstance (Utilities|Casting|CastToBP_Gameinstance (Game|GetGameInstance)))))
    (Rendering|Components|TextRender|SetText (Variables|Default|GetTextRender) (Utilities|Text|ToText(String) (Utilities|String|Append (Utilities|String|ToString(Integer) _count) (Utilities|String|Append " / " (Utilities|String|ToString(Integer) (Variables|Default|GetOrbs%20Needed))))))))

(event Collision|EventActorBeginOverlap
  (params (OtherActor :type Actor%20Object%20Reference)))

(event EventTick
  (params (DeltaSeconds :type Float%20%28single-precision%29))
  (CallFunction|ShowText)
  (bind _count (Default|LoadCollectableCount (.AsBP%20Gameinstance (Utilities|Casting|CastToBP_Gameinstance (Game|GetGameInstance)))))
  (if (< _count (Variables|Default|GetOrbs%20Needed))
    (Variables|Default|SetLocked true)
    (Rendering|Material|SetMaterial (Variables|Default|GetCube) 0 "/Game/Art/Materials/M_EndPointLocked.M_EndPointLocked")
    (else
      (Variables|Default|SetLocked false)
      (Rendering|Material|SetMaterial (Variables|Default|GetCube) 0 "/Game/Art/Materials/M_EndPoint.M_EndPoint")
      (Rendering|Material|SetScalarParameterValueonMaterials (Variables|Default|GetCube) "Hue Shift Percentage (S)" (Variables|Default|GetHue%20Shift)))))

(event EventBeginPlay)

(fn ConstructionScript
  (Rendering|Material|SetScalarParameterValueonMaterials (Variables|Default|GetCube) "Hue Shift Percentage (S)" (Variables|Default|GetHue%20Shift))
  (if (Variables|Default|GetLocked)
    (Rendering|Material|SetMaterial (Variables|Default|GetCube) 0 "/Game/Art/Materials/M_EndPointLocked.M_EndPointLocked")))