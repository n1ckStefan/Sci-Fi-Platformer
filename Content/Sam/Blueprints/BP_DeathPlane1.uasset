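; BP_DeathPlane1 is a kill volume that returns BP_ThirdPersonCharacter to its RespawnPoint when the character overlaps its Collision component.
; After a short delay, it sets the character's JumpCameraZ to the active camera's height and activates the NSFade effect with "Reverse?" set to false.
; A timeline then drives the "Fade" scalar parameter on the character mesh's materials, printing each value to screen.
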(event OnComponentBeginOverlap(Collision)
  (params (OverlappedComponent :type Primitive%20Component%20Object%20Reference) (OtherActor :type Actor%20Object%20Reference) (OtherComp :type Primitive%20Component%20Object%20Reference) (OtherBodyIndex :type Integer) (bFromSweep :type Boolean) (SweepResult :type Hit%20Result%20Structure%20%28by%20ref%29))
  (bind _asbp_third_person_character (Utilities|Casting|CastToBP_ThirdPersonCharacter OtherActor))
  (Transformation|SetActorLocation _asbp_third_person_character (Variables|/Game/ThirdPerson/Blueprints/BP_ThirdPersonCharacter.BP_ThirdPersonCharacter_C|GetRespawnPoint _asbp_third_person_character) false false)
  (Utilities|FlowControl|Delay 0.1)
  (Variables|/Game/ThirdPerson/Blueprints/BP_ThirdPersonCharacter.BP_ThirdPersonCharacter_C|SetJumpCameraZ _asbp_third_person_character (.z (Transformation|GetActorLocation (Variables|/Game/ThirdPerson/Blueprints/BP_ThirdPersonCharacter.BP_ThirdPersonCharacter_C|GetActive%20Camera _asbp_third_person_character))))
  (bind _returnvalue (Actor|GetActorOfClass "/Game/ThirdPerson/Blueprints/BP_ThirdPersonCharacter.BP_ThirdPersonCharacter_C"))
  (Components|Activation|Activate (Variables|/Game/ThirdPerson/Blueprints/BP_ThirdPersonCharacter.BP_ThirdPersonCharacter_C|GetNS_Fade _returnvalue) false)
  (Class|NiagaraComponent|SetVariableBool (Variables|/Game/ThirdPerson/Blueprints/BP_ThirdPersonCharacter.BP_ThirdPersonCharacter_C|GetNS_Fade _returnvalue) "Reverse?" false)
  (bind _newtrack_0 (Timeline|Timeline PlayFromStart)
    (:Update
      (bind _returnvalue_2 (Actor|GetActorOfClass "/Game/ThirdPerson/Blueprints/BP_ThirdPersonCharacter.BP_ThirdPersonCharacter_C"))
      (Rendering|Material|SetScalarParameterValueonMaterials (Variables|/Script/Engine.Character|GetMesh _returnvalue_2) "Fade" _newtrack_0)
      (Development|PrintString (Utilities|String|ToString(Float) _newtrack_0)))))

(event EventBeginPlay)

(event Collision|EventActorBeginOverlap
  (params (OtherActor :type Actor%20Object%20Reference)))

(event EventTick
  (params (DeltaSeconds :type Float%20%28single-precision%29)))

(fn ConstructionScript)