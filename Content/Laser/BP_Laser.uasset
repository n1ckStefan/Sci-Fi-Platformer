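; BP_Laser is a laser hazard that damages and respawns the player character when the beam hits it.
; Each Tick it line-traces between two offsets from the Laser Niagara component's location on the Camera channel.
; A DoOnce with a delayed reset gates ApplyDamage and the Respawn call on BP_ThirdPersonCharacter.
; The construction script passes both offsets and a Kill flag to Niagara, so the effect and trace share endpoint values.
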(event EventBeginPlay)

(event Collision|EventActorBeginOverlap
  (params (OtherActor :type Actor%20Object%20Reference)))

(event EventTick
  (params (DeltaSeconds :type Float%20%28single-precision%29))
  (bind _laser (Variables|Default|GetLaser))
  (bind _returnvalue (Transformation|GetWorldLocation _laser))
  (bind _outhit (Collision|LineTraceByChannel (+ (Variables|Default|GetVector1) _returnvalue) (+ _returnvalue (Variables|Default|GetVector2)) "TraceTypeQuery2" true 0 "None" false))
  (if (== (.HitActor (Collision|BreakHitResult _outhit)) (Game|GetPlayerCharacter 0))
    (bind _asbp_third_person_character (Utilities|Casting|CastToBP_ThirdPersonCharacter (Game|GetPlayerCharacter 0)))
    (Utilities|FlowControl|DoOnce false :!label _label
      (:Completed
        (Game|Damage|ApplyDamage _asbp_third_person_character 1e+01 0 0)
        (Default|Respawn _asbp_third_person_character)
        (Utilities|FlowControl|Delay 1.0)
        (goto _label Reset)))))

(fn ConstructionScript
  (Class|NiagaraComponent|SetNiagaraVariableVec3 (Variables|Default|GetLaser) "Vector1" (Variables|Default|GetVector1))
  (Class|NiagaraComponent|SetNiagaraVariableVec3 (Variables|Default|GetLaser) "Vector2" (Variables|Default|GetVector2))
  (Class|NiagaraComponent|SetVariableBool (Variables|Default|GetLaser) "Kill" (Variables|Default|GetKill)))