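; BP_Enemy is a patrolling enemy that hurts the third-person player character and can be destroyed by it.
; From BeginPlay, it chains AI MoveTo calls through PatrolPoints, but the wrap to index zero does not restart movement, so patrol ends after one pass.
; Overlapping its Attack component launches the player along a fixed vector and applies damage.
; Player overlap with its DeathCondition component destroys the enemy.
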(event OnComponentBeginOverlap(DeathCondition)
  (params (OverlappedComponent :type Primitive%20Component%20Object%20Reference) (OtherActor :type Actor%20Object%20Reference) (OtherComp :type Primitive%20Component%20Object%20Reference) (OtherBodyIndex :type Integer) (bFromSweep :type Boolean) (SweepResult :type Hit%20Result%20Structure%20%28by%20ref%29))
  (Utilities|Casting|CastToBP_ThirdPersonCharacter OtherActor)
  (Actor|DestroyActor))

(event OnComponentBeginOverlap(Attack)
  (params (OverlappedComponent :type Primitive%20Component%20Object%20Reference) (OtherActor :type Actor%20Object%20Reference) (OtherComp :type Primitive%20Component%20Object%20Reference) (OtherBodyIndex :type Integer) (bFromSweep :type Boolean) (SweepResult :type Hit%20Result%20Structure%20%28by%20ref%29))
  (bind _asbp_third_person_character (Utilities|Casting|CastToBP_ThirdPersonCharacter OtherActor))
  (Character|LaunchCharacter _asbp_third_person_character "0.000000,1000.000000,500.000000" false false)
  (Game|Damage|ApplyDamage _asbp_third_person_character 5.0 0 0))

(event Custom|FollowWaypoints
  (AI|AIMoveTo self "0, 0, 0" (Utilities|Array|Get(acopy) (Variables|Default|GetPatrolPoints) (Variables|Default|GetCurrentWaypoint)) 5.0 false
    (:OnSuccess
      (Math|Integer|IncrementInt (Variables|Default|GetCurrentWaypoint)
        (:%20%20
          (if (>= (Variables|Default|GetCurrentWaypoint) (Utilities|Array|Length (Variables|Default|GetPatrolPoints)))
            (Variables|Default|SetCurrentWaypoint 0)
            (else
              (CallFunction|FollowWaypoints))))))))

(event EventBeginPlay
  (CallFunction|FollowWaypoints))

(fn ConstructionScript)