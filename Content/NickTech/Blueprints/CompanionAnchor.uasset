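; CompanionAnchor is a placeable anchor point that the player clicks to set an anchor position for the AI_CompanionNick companion.
; Holding Q reveals the actor and enables the mouse cursor, click and mouse-over events, while releasing Q hides it.
; Clicking MouseCollider passes the anchor's world location to the companion and sets its AnchorSet flag.
; CanWork tracks Q but is never read here, and the nodes that disable the cursor are unwired.
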(event OnClicked(mouseCollider)
  (params (TouchedComponent :type Primitive%20Component%20Object%20Reference) (ButtonPressed :type Key%20Structure :default "None"))
  (bind _returnvalue (Actor|GetActorOfClass "/Game/NickTech/AI/Companion/AI_CompanionNick.AI_CompanionNick_C"))
  (Variables|/Game/NickTech/AI/Companion/AI_CompanionNick.AI_CompanionNick_C|SetanchorSet? _returnvalue true)
  (Variables|/Game/NickTech/AI/Companion/AI_CompanionNick.AI_CompanionNick_C|SetanchorPos _returnvalue (Transformation|GetWorldLocation (Variables|Default|GetcompanionAnchor))))

(event Input|KeyboardEvents|Q
  (params (Key :type Key%20Structure :default "None"))
  (bind _returnvalue (Game|GetPlayerController 0))
  (:Pressed
    (Variables|Default|SetcanWork true)
    (Rendering|SetActorHiddenInGame self false)
    (Variables|/Script/Engine.PlayerController|SetbShowMouseCursor _returnvalue true)
    (Variables|/Script/Engine.PlayerController|SetbEnableClickEvents _returnvalue true)
    (Variables|/Script/Engine.PlayerController|SetbEnableMouseOverEvents _returnvalue true))
  (:Released
    (Variables|Default|SetcanWork false)
    (Rendering|SetActorHiddenInGame self true)))

(fn ConstructionScript)