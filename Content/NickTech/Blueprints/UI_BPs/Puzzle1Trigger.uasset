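; Puzzle1Trigger is a one-shot trigger volume that opens the first puzzle screen when the player character overlaps its box.
; On overlap it freezes global time dilation, clears all widgets and rebuilds the health HUD plus a hidden collectable pop-up, storing the pop-up on BP_ThirdPersonCharacter.
; It then adds WBP_Puzzle1 to the viewport and destroys itself.
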(event OnComponentBeginOverlap(Box)
  (params (OverlappedComponent :type Primitive%20Component%20Object%20Reference) (OtherActor :type Actor%20Object%20Reference) (OtherComp :type Primitive%20Component%20Object%20Reference) (OtherBodyIndex :type Integer) (bFromSweep :type Boolean) (SweepResult :type Hit%20Result%20Structure%20%28by%20ref%29))
  (if (== OtherActor (Game|GetPlayerCharacter 0))
    (Utilities|Time|SetGlobalTimeDilation 0.0)
    (Viewport|RemoveAllWidgets)
    (bind _returnvalue (UserInterface|CreateWidget "/Game/NickTech/UI/WB_Health.WB_Health_C"))
    (bind _returnvalue_2 (UserInterface|CreateWidget "/Game/Sam/Blueprints/Collectables/WBP_CollectablePopUp.WBP_CollectablePopUp_C"))
    (bind _asbp_third_person_character (Utilities|Casting|CastToBP_ThirdPersonCharacter (Game|GetPlayerCharacter 0)))
    (bind _output_get (Variables|/Game/ThirdPerson/Blueprints/BP_ThirdPersonCharacter.BP_ThirdPersonCharacter_C|SetPopUpMenuRef _asbp_third_person_character _returnvalue_2))
    (UserInterface|Viewport|AddtoViewport _returnvalue 0)
    (Widget|SetVisibility (Variables|/Game/ThirdPerson/Blueprints/BP_ThirdPersonCharacter.BP_ThirdPersonCharacter_C|GetPopUpMenuRef _asbp_third_person_character) "Hidden")
    (bind _returnvalue_3 (UserInterface|CreateWidget "/Game/UI/WBP_Puzzle1.WBP_Puzzle1_C"))
    (UserInterface|Viewport|AddtoViewport _returnvalue_3 0)
    (Actor|DestroyActor self)))

(event EventBeginPlay)

(event Collision|EventActorBeginOverlap
  (params (OtherActor :type Actor%20Object%20Reference)))

(event EventTick
  (params (DeltaSeconds :type Float%20%28single-precision%29)))

(fn ConstructionScript)