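; Shaft actor that swings its Pivot component to a fixed rotation once the player enters its Trigger, and removes a BP_QuanttumMatter actor from the level.
; The overlap sets a Triggerable flag that is never cleared, letting Tick ease the pivot with RInterpTo.
; A DoOnce limits the GetActorOfClass lookup and destroy to the first player overlap.
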(event OnComponentBeginOverlap(trigger)
  (params (OverlappedComponent :type Primitive%20Component%20Object%20Reference) (OtherActor :type Actor%20Object%20Reference) (OtherComp :type Primitive%20Component%20Object%20Reference) (OtherBodyIndex :type Integer) (bFromSweep :type Boolean) (SweepResult :type Hit%20Result%20Structure%20%28by%20ref%29))
  (if (== OtherActor (Game|GetPlayerCharacter 0))
    (Variables|Default|Settriggerable true)
    (Utilities|FlowControl|DoOnce false
      (:Completed
        (bind _returnvalue (Actor|GetActorOfClass "/Game/NickTech/Blueprints/BP_QuanttumMatter.BP_QuanttumMatter_C"))
        (Actor|DestroyActor _returnvalue)))))

(event EventTick
  (params (DeltaSeconds :type Float%20%28single-precision%29))
  (bind _pivot (Variables|Default|GetPivot))
  (if (Variables|Default|Gettriggerable)
    (Transformation|SetRelativeRotation _pivot (Math|Interpolation|RInterpTo (Variables|/Script/Engine.SceneComponent|GetRelativeRotation _pivot) "-70.000000,0.000000,0.000000" DeltaSeconds 1.0) false false)))

(fn ConstructionScript)