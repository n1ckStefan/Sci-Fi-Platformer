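; BP_ButtonPlaceHolder is a pressure button that sinks when the player steps on it and counts toward opening a gate.
; A box overlap with the player character sets a trigger flag and, only once, increments ButtonForGate on BP_ThirdPersonCharacter.
; While the flag is set, Tick smoothly interpolates the Button component down to a slightly lowered relative position.
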(event OnComponentBeginOverlap(Box)
  (params (OverlappedComponent :type Primitive%20Component%20Object%20Reference) (OtherActor :type Actor%20Object%20Reference) (OtherComp :type Primitive%20Component%20Object%20Reference) (OtherBodyIndex :type Integer) (bFromSweep :type Boolean) (SweepResult :type Hit%20Result%20Structure%20%28by%20ref%29))
  (if (== OtherActor (Game|GetPlayerCharacter 0))
    (Variables|Default|Settriggerable true)
    (Utilities|FlowControl|DoOnce false
      (:Completed
        (bind _asbp_third_person_character (Utilities|Casting|CastToBP_ThirdPersonCharacter (Game|GetPlayerCharacter 0)))
        (Variables|/Game/ThirdPerson/Blueprints/BP_ThirdPersonCharacter.BP_ThirdPersonCharacter_C|SetButtonForGate _asbp_third_person_character (+ (Variables|/Game/ThirdPerson/Blueprints/BP_ThirdPersonCharacter.BP_ThirdPersonCharacter_C|GetButtonForGate _asbp_third_person_character) 1))))))

(event EventBeginPlay)

(event Collision|EventActorBeginOverlap
  (params (OtherActor :type Actor%20Object%20Reference)))

(event EventTick
  (params (DeltaSeconds :type Float%20%28single-precision%29))
  (bind _button (Variables|Default|Getbutton))
  (if (Variables|Default|Gettriggerable)
    (Transformation|SetRelativeLocation _button (Math|Interpolation|VInterpTo (Variables|/Script/Engine.SceneComponent|GetRelativeLocation _button) "0.000000,0.000000,-1.000000" DeltaSeconds 1.0) false false)))

(fn ConstructionScript)