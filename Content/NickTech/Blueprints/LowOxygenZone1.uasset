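; Low oxygen hazard zone actor that drains the player character's oxygen while they are inside its Box volume.
; Box overlap begin and end swap between looping depletion and recovery timers, each clearing the other, and print debug messages.
; Depletion lowers Oxygen on BP_Character_NickTest without a floor and applies damage each tick at zero or below.
; Recovery refills it faster after exit, stopping at the cap.
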(event OnComponentBeginOverlap(Box)
  (params (OverlappedComponent :type Primitive%20Component%20Object%20Reference) (OtherActor :type Actor%20Object%20Reference) (OtherComp :type Primitive%20Component%20Object%20Reference) (OtherBodyIndex :type Integer) (bFromSweep :type Boolean) (SweepResult :type Hit%20Result%20Structure%20%28by%20ref%29))
  (Development|PrintString "you are in a low oxygen zone")
  (if (== OtherActor (Game|GetPlayerCharacter 0))
    (Utilities|Time|ClearandInvalidateTimerbyHandle (Variables|Default|GetOxygenIncremention))
    (bind _returnvalue (Utilities|Time|SetTimerbyEvent (delegate Custom|DepleteOxygen) 0.2 true))
    (Variables|Default|SetOxygenDepletion _returnvalue)))

(event OnComponentEndOverlap(Box)
  (params (OverlappedComponent :type Primitive%20Component%20Object%20Reference) (OtherActor :type Actor%20Object%20Reference) (OtherComp :type Primitive%20Component%20Object%20Reference) (OtherBodyIndex :type Integer))
  (Development|PrintString "you are no longer in a low oxygen zone")
  (if (== OtherActor (Game|GetPlayerCharacter 0))
    (Utilities|Time|ClearandInvalidateTimerbyHandle (Variables|Default|GetOxygenDepletion))
    (bind _returnvalue (Utilities|Time|SetTimerbyEvent (delegate Custom|IncrementOxygen) 0.2 true))
    (Variables|Default|SetOxygenIncremention _returnvalue)))

(event Custom|DepleteOxygen
  (bind _asbp_character_nick_test (Utilities|Casting|CastToBP_Character_NickTest (Game|GetPlayerCharacter 0)))
  (Variables|/Game/NickTech/Character/BP_Character_NickTest.BP_Character_NickTest_C|SetOxygen _asbp_character_nick_test (- (Variables|/Game/NickTech/Character/BP_Character_NickTest.BP_Character_NickTest_C|GetOxygen _asbp_character_nick_test) 1.0))
  (if (<= (Variables|/Game/NickTech/Character/BP_Character_NickTest.BP_Character_NickTest_C|GetOxygen _asbp_character_nick_test) 0.0)
    (Game|Damage|ApplyDamage _asbp_character_nick_test 1.0 0 0)))

(event Custom|IncrementOxygen
  (bind _asbp_character_nick_test (Utilities|Casting|CastToBP_Character_NickTest (Game|GetPlayerCharacter 0)))
  (Variables|/Game/NickTech/Character/BP_Character_NickTest.BP_Character_NickTest_C|SetOxygen _asbp_character_nick_test (+ (Variables|/Game/NickTech/Character/BP_Character_NickTest.BP_Character_NickTest_C|GetOxygen _asbp_character_nick_test) 5.0))
  (if (>= (Variables|/Game/NickTech/Character/BP_Character_NickTest.BP_Character_NickTest_C|GetOxygen _asbp_character_nick_test) 1e+02)
    (Variables|/Game/NickTech/Character/BP_Character_NickTest.BP_Character_NickTest_C|SetOxygen _asbp_character_nick_test 1e+02)
    (Utilities|Time|ClearandInvalidateTimerbyHandle (Variables|Default|GetOxygenIncremention))))

(event EventBeginPlay)

(event Collision|EventActorBeginOverlap
  (params (OtherActor :type Actor%20Object%20Reference)))

(event EventTick
  (params (DeltaSeconds :type Float%20%28single-precision%29)))

(fn ConstructionScript)