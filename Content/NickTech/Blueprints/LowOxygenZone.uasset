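; Low oxygen hazard zone that drains the player's Oxygen while inside and refills it after exit.
; LowOxygenCollider overlaps swap looping timers that step Oxygen down or up.
; At zero, a DoOnce applies damage, moves the player to RespawnPoint and plays a Niagara and material fade whose timeline re-arms it.
; A separate VisualsCollider drives timelines that fade vignette intensity on the level's first-found PostProcessVolume.
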(event OnComponentBeginOverlap(LowOxygenCollider)
  (params (OverlappedComponent :type Primitive%20Component%20Object%20Reference) (OtherActor :type Actor%20Object%20Reference) (OtherComp :type Primitive%20Component%20Object%20Reference) (OtherBodyIndex :type Integer) (bFromSweep :type Boolean) (SweepResult :type Hit%20Result%20Structure%20%28by%20ref%29))
  (if (== OtherActor (Game|GetPlayerCharacter 0))
    (Utilities|Time|ClearandInvalidateTimerbyHandle (Variables|Default|GetOxygenIncremention))
    (bind _returnvalue (Utilities|Time|SetTimerbyEvent (delegate Custom|DepleteOxygen) 0.2 true))
    (Variables|Default|SetOxygenDepletion _returnvalue)))

(event OnComponentEndOverlap(LowOxygenCollider)
  (params (OverlappedComponent :type Primitive%20Component%20Object%20Reference) (OtherActor :type Actor%20Object%20Reference) (OtherComp :type Primitive%20Component%20Object%20Reference) (OtherBodyIndex :type Integer))
  (if (== OtherActor (Game|GetPlayerCharacter 0))
    (Utilities|Time|ClearandInvalidateTimerbyHandle (Variables|Default|GetOxygenDepletion))
    (bind _returnvalue (Utilities|Time|SetTimerbyEvent (delegate Custom|IncrementOxygen) 0.2 true))
    (Variables|Default|SetOxygenIncremention _returnvalue)))

(event OnComponentBeginOverlap(VisualsCollider)
  (params (OverlappedComponent :type Primitive%20Component%20Object%20Reference) (OtherActor :type Actor%20Object%20Reference) (OtherComp :type Primitive%20Component%20Object%20Reference) (OtherBodyIndex :type Integer) (bFromSweep :type Boolean) (SweepResult :type Hit%20Result%20Structure%20%28by%20ref%29))
  (Variables|Default|SetinZone true)
  (if (== OtherActor (Game|GetPlayerCharacter 0))
    (if (Variables|Default|GetinZone)
      (bind _alpha (Timeline|OxygenFade PlayFromStart)
        (:Update
          (CallFunction|SetPostProcess (* _alpha 1.5))))
      (else
        (Timeline|OxygenFade ReverseFromEnd)))))

(event OnComponentEndOverlap(VisualsCollider)
  (params (OverlappedComponent :type Primitive%20Component%20Object%20Reference) (OtherActor :type Actor%20Object%20Reference) (OtherComp :type Primitive%20Component%20Object%20Reference) (OtherBodyIndex :type Integer))
  (Variables|Default|SetinZone false)
  (if (== OtherActor (Game|GetPlayerCharacter 0))
    (bind _alpha (Timeline|OxygenUnfade PlayFromStart)
      (:Update
        (CallFunction|SetPostProcess (* _alpha 1.5))))))

(event Custom|DepleteOxygen
  (bind _asbp_third_person_character (Utilities|Casting|CastToBP_ThirdPersonCharacter (Game|GetPlayerCharacter 0)))
  (Variables|/Game/ThirdPerson/Blueprints/BP_ThirdPersonCharacter.BP_ThirdPersonCharacter_C|SetOxygen _asbp_third_person_character (- (Variables|/Game/ThirdPerson/Blueprints/BP_ThirdPersonCharacter.BP_ThirdPersonCharacter_C|GetOxygen _asbp_third_person_character) 5.0))
  (if (<= (Variables|/Game/ThirdPerson/Blueprints/BP_ThirdPersonCharacter.BP_ThirdPersonCharacter_C|GetOxygen _asbp_third_person_character) 0.0)
    (Variables|/Game/ThirdPerson/Blueprints/BP_ThirdPersonCharacter.BP_ThirdPersonCharacter_C|SetOxygen _asbp_third_person_character 0.0)
    (Utilities|FlowControl|DoOnce false :!label _label
      (:Completed
        (Game|Damage|ApplyDamage _asbp_third_person_character 2e+01 0 0)
        (bind _asbp_third_person_character_2 (Utilities|Casting|CastToBP_ThirdPersonCharacter (Game|GetPlayerCharacter 0)))
        (Transformation|SetActorLocation _asbp_third_person_character_2 (Variables|/Game/ThirdPerson/Blueprints/BP_ThirdPersonCharacter.BP_ThirdPersonCharacter_C|GetRespawnPoint _asbp_third_person_character_2) false false)
        (Utilities|FlowControl|Delay 0.1)
        (Variables|/Game/ThirdPerson/Blueprints/BP_ThirdPersonCharacter.BP_ThirdPersonCharacter_C|SetJumpCameraZ _asbp_third_person_character_2 (.z (Transformation|GetActorLocation (Variables|/Game/ThirdPerson/Blueprints/BP_ThirdPersonCharacter.BP_ThirdPersonCharacter_C|GetActive%20Camera _asbp_third_person_character_2))))
        (bind _returnvalue (Actor|GetActorOfClass "/Game/ThirdPerson/Blueprints/BP_ThirdPersonCharacter.BP_ThirdPersonCharacter_C"))
        (Components|Activation|Activate (Variables|/Game/ThirdPerson/Blueprints/BP_ThirdPersonCharacter.BP_ThirdPersonCharacter_C|GetNS_Fade _returnvalue) false)
        (Class|NiagaraComponent|SetVariableBool (Variables|/Game/ThirdPerson/Blueprints/BP_ThirdPersonCharacter.BP_ThirdPersonCharacter_C|GetNS_Fade _returnvalue) "Reverse?" false)
        (bind _newtrack_0 (Timeline|Timeline PlayFromStart)
          (:Update
            (bind _returnvalue_2 (Actor|GetActorOfClass "/Game/ThirdPerson/Blueprints/BP_ThirdPersonCharacter.BP_ThirdPersonCharacter_C"))
            (Rendering|Material|SetScalarParameterValueonMaterials (Variables|/Script/Engine.Character|GetMesh _returnvalue_2) "Fade" _newtrack_0)
            (goto _label Reset)))))))

(event Custom|IncrementOxygen
  (bind _asbp_third_person_character (Utilities|Casting|CastToBP_ThirdPersonCharacter (Game|GetPlayerCharacter 0)))
  (Variables|/Game/ThirdPerson/Blueprints/BP_ThirdPersonCharacter.BP_ThirdPersonCharacter_C|SetOxygen _asbp_third_person_character (+ (Variables|/Game/ThirdPerson/Blueprints/BP_ThirdPersonCharacter.BP_ThirdPersonCharacter_C|GetOxygen _asbp_third_person_character) 5.0))
  (if (>= (Variables|/Game/ThirdPerson/Blueprints/BP_ThirdPersonCharacter.BP_ThirdPersonCharacter_C|GetOxygen _asbp_third_person_character) 1e+02)
    (Variables|/Game/ThirdPerson/Blueprints/BP_ThirdPersonCharacter.BP_ThirdPersonCharacter_C|SetOxygen _asbp_third_person_character 1e+02)
    (Utilities|Time|ClearandInvalidateTimerbyHandle (Variables|Default|GetOxygenIncremention))))

(event EventBeginPlay)

(event Collision|EventActorBeginOverlap
  (params (OtherActor :type Actor%20Object%20Reference)))

(event EventTick
  (params (DeltaSeconds :type Float%20%28single-precision%29)))

(fn ConstructionScript)

(fn SetPostProcess
  (params (Vignette :type Float%20%28double-precision%29))
  (bind _returnvalue (Actor|GetActorOfClass "/Script/Engine.PostProcessVolume"))
  (bind _structout (Utilities|Struct|SetmembersinPostProcessSettings (Variables|/Script/Engine.PostProcessVolume|GetSettings _returnvalue) Vignette))
  (Variables|/Script/Engine.PostProcessVolume|SetSettings _returnvalue _structout))