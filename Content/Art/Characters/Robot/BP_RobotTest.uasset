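; Test robot character Blueprint that shows emotions through a face-screen material paired with a Niagara effect.
; SetMaterial maps an emotion index to neutral, shocked, intrigued, angry or hurt visuals, rotating the effect for neutral and hurt.
; Unconnected graph chains would attach Niagara to BoneSocket, pick an emotion from the Oxygen collection parameter, or cycle emotions.
; BeginPlay and Tick are empty, so none of this logic runs from the event graph.
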(event EventBeginPlay)

(event Collision|EventActorBeginOverlap
  (params (OtherActor :type Actor%20Object%20Reference)))

(event EventTick
  (params (DeltaSeconds :type Float%20%28single-precision%29)))

(fn ConstructionScript)

(fn SetMaterial
  (params (NewParam :type Integer))
  (bind _skeletalmesh (Variables|Default|GetSkeletalMesh))
  (if (== NewParam 0)
    (Transformation|SetRelativeRotation (Variables|Default|GetNiagara) "0.000000,0.000000,90.000000" false false)
    (Rendering|Material|SetMaterial _skeletalmesh 0 "/Game/Art/Characters/Robot/Materials/ScreenNeutral.ScreenNeutral")
    (Class|NiagaraComponent|SetAsset (Variables|Default|GetNiagara) "/Game/Art/Niagara/NS_Sleep.NS_Sleep" true)
    (elif (== NewParam 1)
      (Rendering|Material|SetMaterial _skeletalmesh 0 "/Game/Art/Characters/Robot/Materials/ScreenShocked.ScreenShocked")
      (Class|NiagaraComponent|SetAsset (Variables|Default|GetNiagara) "/Game/Art/Niagara/NS_Exclamation.NS_Exclamation" true)
      (elif (== NewParam 2)
        (Rendering|Material|SetMaterial _skeletalmesh 0 "/Game/Art/Characters/Robot/Materials/ScreenIntruiged.ScreenIntruiged")
        (Class|NiagaraComponent|SetAsset (Variables|Default|GetNiagara) "/Game/Art/Niagara/NS_Question.NS_Question" true)
        (elif (== NewParam 3)
          (Rendering|Material|SetMaterial _skeletalmesh 0 "/Game/Art/Characters/Robot/Materials/ScreenAngry.ScreenAngry")
          (Class|NiagaraComponent|SetAsset (Variables|Default|GetNiagara) "/Game/Art/Niagara/NS_Angry.NS_Angry" true)
          (else
            (Rendering|Material|SetMaterial _skeletalmesh 0 "/Game/Art/Characters/Robot/Materials/ScreenHurt.ScreenHurt")
            (Class|NiagaraComponent|SetAsset (Variables|Default|GetNiagara) "/Game/Art/Niagara/NS_Cry.NS_Cry" true)
            (Transformation|SetRelativeRotation (Variables|Default|GetNiagara) "90.000000,0.000000,90.000000" false false)))))))