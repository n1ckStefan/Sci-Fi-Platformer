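; BP_Ground is a ground piece made of a main Ground component with left and right corner components, configured in the construction script.
; A boolean per corner hides that corner when set to true.
; A Colour selector applies one of three materials to all three components: two desert ground instances or M_Ground.
; The event graph holds only disabled default events, so it adds no runtime logic.
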(event EventBeginPlay)

(event Collision|EventActorBeginOverlap
  (params (OtherActor :type Actor%20Object%20Reference)))

(event EventTick
  (params (DeltaSeconds :type Float%20%28single-precision%29)))

(fn ConstructionScript
  (if (== (Variables|Default|GetConrnerR?) false)
    _
    (else
      (Rendering|SetVisibility (Variables|Default|GetCornerR) false false)))
  (if (== (Variables|Default|GetCornerL?) false)
    _
    (else
      (Rendering|SetVisibility (Variables|Default|GetCornerL) false false)))
  (if (== (Variables|Default|GetColour) 0)
    (Rendering|Material|SetMaterial (Variables|Default|GetGround) 0 "/Game/Art/Materials/ground/MI_GroundDesert1.MI_GroundDesert1")
    (elif (== (Variables|Default|GetColour) 1)
      (Rendering|Material|SetMaterial (Variables|Default|GetGround) 0 "/Game/Art/Materials/ground/MI_GroundDesert.MI_GroundDesert")
      (elif (== (Variables|Default|GetColour) 2)
        (Rendering|Material|SetMaterial (Variables|Default|GetGround) 0 "/Game/Art/Materials/ground/M_Ground.M_Ground")))))