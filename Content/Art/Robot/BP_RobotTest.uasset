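; BP_RobotTest is a test robot actor that shows emotions through screen materials paired with Niagara effects.
; BeginPlay snaps the effect to BoneSocket, then picks neutral or intrigued from the Oxygen parameter collection value.
; SetMaterial maps an index to a face and effect.
; Tick cycles Emotion through four states every frame, while its trailing two-second Delay resets only the screen to neutral.
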(event EventBeginPlay
  (Transformation|AttachComponentToComponent (Variables|Default|GetNiagara) 0 "BoneSocket" "SnapToTarget" "KeepWorld" "KeepWorld" true)
  (bind _returnvalue (Rendering|Material|GetScalarParameterValue "/Game/Art/OxygenParameters.OxygenParameters" "Oxygen" :!class /Script/Engine.KismetMaterialLibrary))
  (if (> _returnvalue 0.5)
    (CallFunction|SetMaterial)
    (else
      (CallFunction|SetMaterial 2))))

(event Collision|EventActorBeginOverlap
  (params (OtherActor :type Actor%20Object%20Reference)))

(event EventTick
  (params (DeltaSeconds :type Float%20%28single-precision%29))
  (Components|Activation|Activate (Variables|Default|GetNiagara) false)
  (bind _output_get (Variables|Default|SetEmotion (+ (Variables|Default|GetEmotion) 1)))
  (if (> _output_get 3)
    (bind _output_get_2 (Variables|Default|SetEmotion 0))
    (CallFunction|SetMaterial _output_get_2)
    (else
      (CallFunction|SetMaterial _output_get)))
  (Utilities|FlowControl|Delay 2.0)
  (Rendering|Material|SetMaterial (Variables|Default|GetSkeletalMesh) 0 "/Game/Art/Robot/Materials/ScreenNeutral.ScreenNeutral"))

(fn ConstructionScript)

(fn SetMaterial
  (params (NewParam :type Integer))
  (bind _skeletalmesh (Variables|Default|GetSkeletalMesh))
  (if (== NewParam 0)
    (Rendering|Material|SetMaterial _skeletalmesh 0 "/Game/Art/Robot/Materials/ScreenNeutral.ScreenNeutral")
    (Class|NiagaraComponent|SetAsset (Variables|Default|GetNiagara) "/Game/Art/Niagara/NS_Sleep.NS_Sleep" true)
    (elif (== NewParam 1)
      (Rendering|Material|SetMaterial _skeletalmesh 0 "/Game/Art/Robot/Materials/ScreenShocked.ScreenShocked")
      (Class|NiagaraComponent|SetAsset (Variables|Default|GetNiagara) "/Game/Art/Niagara/NS_Exclamation.NS_Exclamation" true)
      (elif (== NewParam 2)
        (Rendering|Material|SetMaterial _skeletalmesh 0 "/Game/Art/Robot/Materials/ScreenIntruiged.ScreenIntruiged")
        (Class|NiagaraComponent|SetAsset (Variables|Default|GetNiagara) "/Game/Art/Niagara/NS_Question.NS_Question" true)
        (elif (== NewParam 3)
          (Rendering|Material|SetMaterial _skeletalmesh 0 "/Game/Art/Robot/Materials/ScreenAngry.ScreenAngry")
          (Class|NiagaraComponent|SetAsset (Variables|Default|GetNiagara) "/Game/Art/Niagara/NS_Angry.NS_Angry" true)
          (else
            (Rendering|Material|SetMaterial _skeletalmesh 0 "/Game/Art/Robot/Materials/ScreenHurt.ScreenHurt")
            (Class|NiagaraComponent|SetAsset (Variables|Default|GetNiagara) "/Game/Art/Niagara/NS_Sweat.NS_Sweat" true)))))))