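; BP_OxygenVolume is a placeable volume that drives an "Oxygen" material parameter on nearby mushrooms.
; Its construction script gathers every BP_Mushroom and checks each mesh's distance from the volume's Sphere.
; Meshes within Range get the Oxygen value set as a scalar on their materials.
; The work happens only at construction; the event graph has no active logic.
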(event EventBeginPlay)

(event Collision|EventActorBeginOverlap
  (params (OtherActor :type Actor%20Object%20Reference)))

(event EventTick
  (params (DeltaSeconds :type Float%20%28single-precision%29)))

(fn ConstructionScript
  (bind _outactors (Actor|GetAllActorsOfClass "/Game/Art/Environment/mushroom/BP_Mushroom.BP_Mushroom_C"))
  (for _array_element _outactors
    (if (<= (Math|Float|Absolute(Float) (Math|Vector|Distance(Vector) (Transformation|GetWorldLocation (Variables|Default|GetSphere)) (Transformation|GetWorldLocation (Variables|/Game/Art/Environment/mushroom/BP_Mushroom.BP_Mushroom_C|GetStaticMesh _array_element)))) (Variables|Default|GetRange))
      (Rendering|Material|SetScalarParameterValueonMaterials (Variables|/Game/Art/Environment/mushroom/BP_Mushroom.BP_Mushroom_C|GetStaticMesh _array_element) "Oxygen" (Variables|Default|GetOxygen)))))